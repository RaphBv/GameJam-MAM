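; BP_Moderation is a moderation gameplay actor that follows the player's BP_Jean pawn until it is provoked.
; After a short delay at BeginPlay, it caches the player and starts a looping timer that drives movement instead of Tick.
; Each update moves it toward the player with a swept step, turns it to face them, and stops within follow distance.
; When IsProvoked is set, OnPlayerProvoked clears the timer once, ending the follow.
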(event `self.ReceiveBeginPlay`
  (`self.PlayerToFollow`
    (:`then`)
    (:`else`
      (`KismetSystemLibrary.Delay` 0.2)
      (`self.SetTargetPlayer` (`GameplayStatics.GetPlayerPawn` 0))
      (bind _returnvalue (`KismetSystemLibrary.K2_SetTimerDelegate` (delegate `UpdateFollow`) (`self.UpdateRate`) true))
      (set `self.FollowTimer` _returnvalue))))

(event `UpdateFollow`
  (if (`self.IsProvoked`)
    (`/Engine/EditorBlueprintResources/StandardMacros.DoOnce` false
      (:`Completed`
        (`self.OnPlayerProvoked`)))
    (else
      (`self.PlayerToFollow`
        (:`then`
          (set `self.Direction` (- (`self.K2_GetActorLocation` (`self.PlayerToFollow`)) (`self.K2_GetActorLocation`)))
          (set `self.Distance` (`KismetMathLibrary.VSize` (`self.Direction`)))
          (if (<= (`self.Distance`) (`self.FollowDistance`))
            (set `self.isMoving` false)
            (else
              (set `self.isMoving` true)
              (`self.K2_SetActorLocation` (+ (`self.K2_GetActorLocation`) (* (`KismetMathLibrary.Normal` (`self.Direction`)) (`self.MoveSpeed`) (`self.UpdateRate`))) true)
              (`self.K2_SetActorRotation` (`KismetMathLibrary.FindLookAtRotation` (`self.K2_GetActorLocation`) (`self.K2_GetActorLocation` (`self.PlayerToFollow`)))))))
        (:`else`)))))

(fn `OnPlayerProvoked`
  (if (`KismetSystemLibrary.K2_IsTimerActiveHandle` (`self.FollowTimer`))
    (`KismetSystemLibrary.K2_ClearAndInvalidateTimerHandle` (`self.FollowTimer`))))

(fn `SetTargetPlayer`
  (params (Player :type "Actor Object Reference"))
  (bind _asbp_jean (cast `/Game/Blueprint/3C/Player/BP_Jean` Player))
  (set `self.PlayerToFollow` _asbp_jean))

(fn `UserConstructionScript`)