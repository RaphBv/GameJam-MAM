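; Game mode that runs a timed round and picks an ending from the state of the level's BP_Events actors.
; A looping one-second timer counts RemainingTime down and calls EndGame at zero, which switches to UI input with a cursor.
; EndGame shows the lose, middle "Couch" or win widget by the share of events flagged IsGood.
; Tick scans all events and cuts RemainingTime short when none are good.
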(event `self.ReceiveTick`
  (params (DeltaSeconds :type "Float (single-precision)"))
  (`self.CheckIfNotGood`))

(event `self.ReceiveBeginPlay`
  ;[0.04478 0.15 0 0.5] Set Game Timer
  (set `self.RemainingTime` (`self.TotalTime`))
  (bind _returnvalue (`KismetSystemLibrary.K2_SetTimerDelegate` (delegate `TimerEvent`) 1.0 true))
  (set `self.GameTimer` _returnvalue))

(event `TimerEvent`
  ;[0.002707 0.15 0 0.5] Timer Event
  (set `self.RemainingTime` (- (`self.RemainingTime`) 1))
  (if (<= (`self.RemainingTime`) 0)
    (`KismetSystemLibrary.K2_ClearAndInvalidateTimerHandle` (`self.GameTimer`))
    (set `self.RemainingTime` 0)
    (`self.EndGame`)))

(fn `CheckIfNotGood`
  (locals (Total :type Integer) (NotGood :type Integer))
  (bind _outactors (`GameplayStatics.GetAllActorsOfClass` "/Game/Blueprint/GPE/Events/BP_Events.BP_Events_C"))
  (for _array_element _outactors
    (if (not (`/Game/Blueprint/GPE/Events/BP_Events.IsGood` _array_element))
      (`/Engine/EditorBlueprintResources/StandardMacros.IncrementInt` (`local.NotGood`)
        (:`  `
          _)))
    (`/Engine/EditorBlueprintResources/StandardMacros.IncrementInt` (`local.Total`)))
  (if (== (`local.NotGood`) (`local.Total`))
    (set `self.RemainingTime` 1)))

(fn `Couch`
  (bind _returnvalue (`|CreateWidget` "/Game/Blueprint/Widget/UW_Couch.UW_Couch_C"))
  (`UserWidget.AddToViewport` _returnvalue 0))

(fn `EndGame`
  (locals (Percent :type "Float (double-precision)"))
  (bind _returnvalue (`GameplayStatics.GetPlayerController` 0))
  (`KismetSystemLibrary.PrintString` "FINNNNNNNNNNNNNNNNNNNNNNNN")
  (`WidgetBlueprintLibrary.SetInputMode_UIOnlyEx` _returnvalue null)
  (set `PlayerController.bShowMouseCursor` true _returnvalue)
  (bind _outactors (`GameplayStatics.GetAllActorsOfClass` "/Game/Blueprint/GPE/Events/BP_Events.BP_Events_C"))
  (set `self.AllEvents` _outactors)
  (for _array_element (`self.AllEvents`)
    (if (`/Game/Blueprint/GPE/Events/BP_Events.IsGood` _array_element)
      (`/Engine/EditorBlueprintResources/StandardMacros.IncrementInt` (`self.Suceeded`)
        (:`  `
          _)))
    (`/Engine/EditorBlueprintResources/StandardMacros.IncrementInt` (`self.TotalEvents`)))
  (set `local.Percent` (/ (`self.Suceeded`) (`self.TotalEvents`)))
  (if (< (`local.Percent`) 0.3)
    (`self.Loose`)
    (`KismetSystemLibrary.PrintString` "LOOOOOOOOOOOOOOOOOOOOOOSE")
    (elif (> (`local.Percent`) 0.7)
      (`self.Win`)
      (`KismetSystemLibrary.PrintString` "WIIIIIIIINNNNNNNNNNNNNNNNNNNNNNNNNNNNNNNNNNNN")
      (else
        (`self.Couch`)
        (`KismetSystemLibrary.PrintString` "COUCHHHHHHHHHHHHHHHHHHHHHHHHHHHHHHHHHH")))))

(fn `Loose`
  (bind _returnvalue (`|CreateWidget` "/Game/Blueprint/Widget/UW_Lose.UW_Lose_C"))
  (`UserWidget.AddToViewport` _returnvalue 0))

(fn `UserConstructionScript`)

(fn `Win`
  (bind _returnvalue (`|CreateWidget` "/Game/Blueprint/Widget/UW_Win.UW_Win_C"))
  (`UserWidget.AddToViewport` _returnvalue 0))