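; BP_Events is an interactable gameplay event that the player resolves by using a required item.
; Interact checks BP_Jean's active inventory item against ItemNeeded; a match destroys the item, sets IsGood, plays a success sound and stops the Niagara effect.
; A mismatch plays a failure sound, and a resolved event ignores further interaction.
; SetActivated stores an activation flag not read here, and ActivateFX starts the effect.
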(event `self.ReceiveTick`
  (params (DeltaSeconds :type "Float (single-precision)")))

(fn `ActivateFX`
  (`ActorComponent.Activate` (`self.Niagara`) false))

(fn `Interact`
  (params (Player :type "Character Object Reference"))
  (if (not (`self.IsGood`))
    (bind _asbp_jean (cast `/Game/Blueprint/3C/Player/BP_Jean` Player))
    (bind _bp_inventorycomponent (`/Game/Blueprint/3C/Player/BP_Jean.BP_InventoryComponent` _asbp_jean))
    (if (== (`/Game/Blueprint/3C/Inventory/BP_InventoryComponent.ActiveItem` _bp_inventorycomponent) (`self.ItemNeeded`))
      (`/Game/Blueprint/3C/Inventory/BP_InventoryComponent.DropActiveItemAndDestroy` _bp_inventorycomponent)
      (set `self.IsGood` true)
      (`GameplayStatics.PlaySound2D` "/Engine/EditorSounds/Notifications/CompileSuccess.CompileSuccess" 1.0 1.0 0.0 null null)
      (bind _niagara (`self.Niagara`)
        (:`then`
          (`ActorComponent.Deactivate` _niagara))
        (:`else`))
      (else
        (set `self.IsGood` false)
        (`GameplayStatics.PlaySound2D` "/Engine/EditorSounds/Notifications/CompileFailed.CompileFailed" 1.0 1.0 0.0 null null)))))

(fn `SetActivated`
  (params (IsActivated :type Boolean))
  (set `self.IsActivated` IsActivated))

(fn `UserConstructionScript`)