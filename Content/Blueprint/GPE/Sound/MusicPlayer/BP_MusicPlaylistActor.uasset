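; Playlist actor that plays the sounds in MusicList one after another, starting from the first at BeginPlay.
; PlayCurrentMusic sets the current sound on the Audio component, plays it at low volume and starts a timer matching its duration.
; CurrentMusic advances the index with wraparound to loop the list and replays.
; An audio-finished handler does the same, but its binding never runs; debug prints remain.
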(event `self.ReceiveBeginPlay`
  (set `self.CurrentIndex` 0)
  (`self.PlayCurrentMusic`))

(event `CurrentMusic`
  (set `self.CurrentIndex` (mod (+ (`self.CurrentIndex`) 1) (`KismetArrayLibrary.Array_Length` (`self.MusicList`))))
  (`self.PlayCurrentMusic`)
  (`KismetSystemLibrary.PrintString` "YESSSSSSSSSS"))

(event `OnAudioFinished_Event`
  (set `self.CurrentIndex` (mod (+ (`self.CurrentIndex`) 1) (`KismetArrayLibrary.Array_Length` (`self.MusicList`))))
  (`self.PlayCurrentMusic`)
  (`KismetSystemLibrary.PrintString` "Finish"))

(fn `PlayCurrentMusic`
  (bind _audio (`self.Audio`))
  (if (`KismetArrayLibrary.Array_IsNotEmpty` (`self.MusicList`))
    (bind _output_get (set `self.CurrentSound` (`|GetArrayItem` (`self.MusicList`) (`self.CurrentIndex`))))
    (`AudioComponent.SetSound` (`self.Audio`) _output_get)
    (`AudioComponent.Play` _audio 0.0)
    (`AudioComponent.SetVolumeMultiplier` _audio 0.1)
    (bind _output_get_2 (set `self.TrackDuration` (`SoundBase.Duration` (`self.CurrentSound`))))
    (bind _returnvalue (`KismetSystemLibrary.K2_SetTimerDelegate` (`|CreateDelegate` :!event `CurrentMusic`) _output_get_2))
    (set `self.TrackTimerHandle` _returnvalue)
    (`KismetSystemLibrary.PrintString` "Hello")))

(fn `UserConstructionScript`)