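; Inventory component for BP_Jean that picks up, cycles, drops and destroys carried items.
; Pickup checks both total weight and item count against MaxHeight, then disables the item's physics and collision.
; AttachActiveItem snaps the active item's mesh to its socket on Jean's mesh and hides the others.
; Dropping launches BP_PNJ items forward with an impulse, sets others down offset without physics, and plays Jean's throw animation.
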(event `DelayEvent`
  (params (Delay :type "Float (double-precision)"))
  (`KismetSystemLibrary.Delay` Delay))

(fn `AttachActiveItem`
  (locals (Item :type "/Game/Blueprint/GPE/Items/BP_BaseItem Object Reference") (RelativeScale :type "Vector Structure"))
  (bind _item (`local.Item`))
  (if (== (`KismetArrayLibrary.Array_Length` (`self.Inventory`)) 0)
    (set `self.ActiveItem` null)
    (else
      (if (not (`KismetArrayLibrary.Array_IsValidIndex` (`self.Inventory`) (`self.ActiveItemIndex`)))
        (set `self.ActiveItemIndex` 0))
      (set `local.Item` (`|GetArrayItem` (`self.Inventory`) (`self.ActiveItemIndex`)))
      (bind _asbp_jean (cast `/Game/Blueprint/3C/Player/BP_Jean` (`self.GetOwner`)))
      (`/Engine/EditorBlueprintResources/StandardMacros.IsValid` _item
        (:`Is Valid`
          (set `local.RelativeScale` (/ (`Actor.GetActorScale3D` _item) 100.0))
          (bind _returnvalue (`SceneComponent.K2_AttachToComponent` (`/Game/Blueprint/GPE/Items/BP_BaseItem.StaticMesh` _item) (`Character.Mesh` _asbp_jean) (`/Game/Blueprint/GPE/Items/BP_BaseItem.AttachSocket` _item) "SnapToTarget" "SnapToTarget" "SnapToTarget" false))
          (`SceneComponent.SetRelativeScale3D` (`/Game/Blueprint/GPE/Items/BP_BaseItem.StaticMesh` (`local.Item`)) (`local.RelativeScale`))
          (set `self.ActiveItem` (`|GetArrayItem` (`self.Inventory`) (`self.ActiveItemIndex`)))
          (for _array_element (`self.Inventory`)
            (if (== _array_element (`self.ActiveItem`))
              (bind _staticmesh (`/Game/Blueprint/GPE/Items/BP_BaseItem.StaticMesh` _array_element))
              (`SceneComponent.SetVisibility` _staticmesh true false)
              (else
                (`SceneComponent.SetVisibility` _staticmesh false false))))
          (if _returnvalue
            (`KismetSystemLibrary.PrintString` "SUCCESSS")
            (else
              (`KismetSystemLibrary.PrintString` "LOOSEEEEEEEEEEEEEEEEEEEEEE"))))))))

(fn `DropActiveItem`
  (locals (Item :type "/Game/Blueprint/GPE/Items/BP_BaseItem Object Reference"))
  (bind _item (`local.Item`))
  (bind _output (`|GetArrayItem` (`self.Inventory`) (`self.ActiveItemIndex`)))
  (bind _staticmesh (`/Game/Blueprint/GPE/Items/BP_BaseItem.StaticMesh` _item))
  (bind (_relativelocation_x _relativelocation_y) (`KismetMathLibrary.BreakVector` (`SceneComponent.RelativeLocation` _staticmesh)))
  (if (not (== (`KismetArrayLibrary.Array_Length` (`self.Inventory`)) 0))
    (`/Engine/EditorBlueprintResources/StandardMacros.IsValid` _output
      (:`Is Valid`
        (bind _output_get (set `local.Item` _output))
        (`SceneComponent.K2_DetachFromComponent` (`/Game/Blueprint/GPE/Items/BP_BaseItem.StaticMesh` _output_get) "KeepWorld" "KeepWorld" "KeepWorld" true)
        (if (`KismetMathLibrary.ClassIsChildOf` (`GameplayStatics.GetObjectClass` _item) "/Game/Blueprint/GPE/Items/PNJ/BP_PNJ.BP_PNJ_C")
          (`KismetSystemLibrary.PrintString` "PNJJJJJJJJJJJJJ")
          (`PrimitiveComponent.SetSimulatePhysics` _staticmesh true)
          (`PrimitiveComponent.SetCollisionEnabled` _staticmesh "QueryAndPhysics")
          (`PrimitiveComponent.AddImpulse` _staticmesh (* (`Actor.GetActorForwardVector` (`self.GetOwner`)) (`self.Force`)) "None" true)
          (`KismetArrayLibrary.Array_Remove` (`self.Inventory`) (`self.ActiveItemIndex`))
          (if (<= (`self.ActiveItemIndex`) (`KismetArrayLibrary.Array_Length` (`self.Inventory`)))
            (set `self.ActiveItemIndex` (`KismetMathLibrary.Max` 0 (- (`KismetArrayLibrary.Array_Length` (`self.Inventory`)) 1))))
          (`self.AttachActiveItem`)
          (bind _asbp_jean (cast `/Game/Blueprint/3C/Player/BP_Jean` (`self.GetOwner`)))
          (`/Game/Blueprint/3C/Player/BP_Jean.ThrowAnim` _asbp_jean)
          (else
            (`PrimitiveComponent.SetSimulatePhysics` _staticmesh false)
            (`PrimitiveComponent.SetCollisionEnabled` _staticmesh "QueryAndPhysics")
            (`SceneComponent.K2_SetRelativeLocation` _staticmesh (`KismetMathLibrary.MakeVector` (+ _relativelocation_x 100.0) _relativelocation_y) false false)
            (`KismetArrayLibrary.Array_Remove` (`self.Inventory`) (`self.ActiveItemIndex`))
            (if (<= (`self.ActiveItemIndex`) (`KismetArrayLibrary.Array_Length` (`self.Inventory`)))
              (set `self.ActiveItemIndex` (`KismetMathLibrary.Max` 0 (- (`KismetArrayLibrary.Array_Length` (`self.Inventory`)) 1))))
            (`self.AttachActiveItem`)
            (bind _asbp_jean_2 (cast `/Game/Blueprint/3C/Player/BP_Jean` (`self.GetOwner`)))
            (`/Game/Blueprint/3C/Player/BP_Jean.ThrowAnim` _asbp_jean_2)))))))

(fn `DropActiveItemAndDestroy`
  (locals (Item :type "/Game/Blueprint/GPE/Items/BP_BaseItem Object Reference"))
  (bind _output (`|GetArrayItem` (`self.Inventory`) (`self.ActiveItemIndex`)))
  (if (not (== (`KismetArrayLibrary.Array_Length` (`self.Inventory`)) 0))
    (`/Engine/EditorBlueprintResources/StandardMacros.IsValid` _output
      (:`Is Valid`
        (bind _output_get (set `local.Item` _output))
        (`SceneComponent.K2_DetachFromComponent` (`/Game/Blueprint/GPE/Items/BP_BaseItem.StaticMesh` _output_get) "KeepWorld" "KeepWorld" "KeepWorld" true)
        (`Actor.K2_DestroyActor` (`local.Item`))
        (`KismetArrayLibrary.Array_Remove` (`self.Inventory`) (`self.ActiveItemIndex`))
        (if (<= (`self.ActiveItemIndex`) (`KismetArrayLibrary.Array_Length` (`self.Inventory`)))
          (set `self.ActiveItemIndex` (`KismetMathLibrary.Max` 0 (- (`KismetArrayLibrary.Array_Length` (`self.Inventory`)) 1))))
        (`self.AttachActiveItem`)
        (bind _asbp_jean (cast `/Game/Blueprint/3C/Player/BP_Jean` (`self.GetOwner`)))
        (`/Game/Blueprint/3C/Player/BP_Jean.ThrowAnim` _asbp_jean)))))

(fn `GetTotalWeight`
  (returns (TotalWeight :type Integer))
  (locals (Total :type Integer))
  (set `local.Total` 0)
  (for _array_element (`self.Inventory`)
    (`/Engine/EditorBlueprintResources/StandardMacros.IsValid` _array_element
      (:`Is Valid`
        (set `local.Total` (+ (`/Game/Blueprint/GPE/Items/BP_BaseItem.Weight` _array_element) (`local.Total`))))))
  (return (`local.Total`)))

(fn `NextItem`
  (set `self.ActiveItemIndex` (+ (`self.ActiveItemIndex`) 1))
  (if (>= (`self.ActiveItemIndex`) (`KismetArrayLibrary.Array_Length` (`self.Inventory`)))
    (set `self.ActiveItemIndex` 0))
  (`self.AttachActiveItem`))

(fn `PickupItem`
  (params (Item :type "/Game/Blueprint/GPE/Items/BP_BaseItem Object Reference"))
  (returns (CanPickup :type Boolean))
  (bind _staticmesh (`/Game/Blueprint/GPE/Items/BP_BaseItem.StaticMesh` Item))
  (`/Engine/EditorBlueprintResources/StandardMacros.IsValid` Item
    (:`Is Valid`
      (if (not (> (+ (`self.GetTotalWeight`) (`/Game/Blueprint/GPE/Items/BP_BaseItem.Weight` Item)) (`self.MaxHeight`)))
        (if (not (>= (`KismetArrayLibrary.Array_Length` (`self.Inventory`)) (`self.MaxHeight`)))
          (`KismetArrayLibrary.Array_Add` (`self.Inventory`) Item)
          (`PrimitiveComponent.SetSimulatePhysics` _staticmesh false)
          (`PrimitiveComponent.SetCollisionEnabled` _staticmesh "NoCollision")
          (`self.AttachActiveItem`)
          (bind _asbp_jean (cast `/Game/Blueprint/3C/Player/BP_Jean` (`self.GetOwner`))
            (:`then`
              (`/Game/Blueprint/3C/Player/BP_Jean.PickUpAnim` _asbp_jean))
            (:`CastFailed`
              _))
          (return true)
          (else
            (return false)))
        (else
          (return false))))
    (:`Is Not Valid`
      (return false))))

(fn `PreviousItem`
  (set `self.ActiveItemIndex` (- (`self.ActiveItemIndex`) 1))
  (if (< (`self.ActiveItemIndex`) 0)
    (set `self.ActiveItemIndex` (- (`KismetArrayLibrary.Array_Length` (`self.Inventory`)) 1)))
  (`self.AttachActiveItem`))