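; BP_Fridge is an interactive fridge whose door swings open when BP_Jean enters its trigger box and can reveal a linked Item.
; The OpenClose timeline lerps the door's yaw on overlap and reverses when any actor leaves the box, with no cast on exit.
; A valid Item has its mesh hidden at BeginPlay, then shown through a DoOnce when the timeline finishes.
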(event `self.ReceiveBeginPlay`
  (bind _item (`self.Item`))
  (`/Engine/EditorBlueprintResources/StandardMacros.IsValid` _item
    (:`Is Valid`
      (`SceneComponent.SetVisibility` (`/Game/Blueprint/GPE/Items/BP_BaseItem.StaticMesh` _item) false false))))

(event `self.Box.OnComponentBeginOverlap`
  (params (OverlappedComponent :type "PrimitiveComponent Object Reference") (OtherActor :type "Actor Object Reference") (OtherComp :type "PrimitiveComponent Object Reference") (OtherBodyIndex :type Integer) (bFromSweep :type Boolean) (SweepResult :type "HitResult Structure (by ref)"))
  (bind _door (`self.Door`))
  (bind (_relativerotation_roll _relativerotation_pitch) (`KismetMathLibrary.BreakRotator` (`SceneComponent.RelativeRotation` _door)))
  (cast `/Game/Blueprint/3C/Player/BP_Jean` OtherActor)
  (bind (_direction _newtrack_0) (`Timeline|Open/Close` :!label _label)
    (:`Update`
      (`SceneComponent.K2_SetRelativeRotation` _door (`KismetMathLibrary.MakeRotator` _relativerotation_roll _relativerotation_pitch (`KismetMathLibrary.Lerp` -90.0 -180.0 _newtrack_0)) false false))
    (:`Finished`
      (bind _item (`self.Item`)
        (:`then`
          (`/Engine/EditorBlueprintResources/StandardMacros.DoOnce` false
            (:`Completed`
              (`SceneComponent.SetVisibility` (`/Game/Blueprint/GPE/Items/BP_BaseItem.StaticMesh` _item) true false))))
        (:`else`)))))

(event `self.Box.OnComponentEndOverlap`
  (params (OverlappedComponent :type "PrimitiveComponent Object Reference") (OtherActor :type "Actor Object Reference") (OtherComp :type "PrimitiveComponent Object Reference") (OtherBodyIndex :type Integer))
  (goto _label :!via `Reverse`))

(fn `UserConstructionScript`)